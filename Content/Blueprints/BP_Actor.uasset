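; BP_Actor is a pawn that wanders endlessly between random points inside a rectangular area sized from Min/Max X and Y bounds.
; BeginPlay applies Speed to FloatingPawnMovement and starts MoveToPoint, which runs AI MoveTo and calls itself with a new point on success, or on failure while inside.
; A zero-Delay loop records the last in-box location; upon leaving the box, it stops movement and sends the pawn back there.
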(event Custom|MoveToPoint
  (params (Target :type Vector) (Back :type Boolean) (Radius :type Float%20%28double-precision%29))
  (bind _returnvalue (Transformation|GetActorLocation))
  (bind _returnvalue_2 (|(((Abs({2F66DE7D-4700-A58F-BFAA-8380BBD5154D}))+(Abs({672AA9A6-45E3-BEA2-7B3E-229BD895330A})))/2)))
  (bind _returnvalue_3 (|(((Abs({FB4D8B70-4EC4-0B5F-75BD-5B8731465C87}))+(Abs({1ED38B1F-4DC4-F434-B221-8396986A2B4B})))/2)))
  (bind _returnvalue_4 (Math|Geometry|IsPointinBox _returnvalue "0, 0, 0" (Math|Vector|MakeVector _returnvalue_3 _returnvalue_2 1e+02)))
  ;[0 0 0] Движение актора в заданную точку, вызов этой же функции с другой точкой
  (AI|AIMoveTo self Target 0 Radius false
    (:then
      ;[0 0 0] Возвращение актора в последнюю точку в зоне, если он вышел из неё, иначе перезапись последней локации актора
      (Utilities|FlowControl|Delay 0.0 :!label _label)
      (if (or Back _returnvalue_4)
        (Variables|Default|SetPreviosLocation (Math|Vector|SelectVector (Transformation|GetActorLocation) (Variables|Default|GetPreviosLocation) _returnvalue_4))
        (Variables|Default|SetActorInBox true)
        (goto _label)
        (else
          (Variables|Default|SetActorInBox false)
          (Components|Movement|StopMovementImmediately (Variables|Default|GetFloatingPawnMovement))
          (CallFunction|MovetoPoint (Variables|Default|GetPreviosLocation) true 0.01))))
    (:OnSuccess
      (CallFunction|MovetoPoint (Math|Random|RandomPointinBoundingBox "0, 0, 0" (Math|Vector|MakeVector (|(((Abs({FB4D8B70-4EC4-0B5F-75BD-5B8731465C87}))+(Abs({1ED38B1F-4DC4-F434-B221-8396986A2B4B})))/2)) (|(((Abs({2F66DE7D-4700-A58F-BFAA-8380BBD5154D}))+(Abs({672AA9A6-45E3-BEA2-7B3E-229BD895330A})))/2)) 0.0)) false 1e+01 :!label _label_2))
    (:OnFail
      (if (Variables|Default|GetActorInBox)
        (goto _label_2)))))

(event EventBeginPlay
  ;[0 0 0] Запись начальной локации, скорости, вызов AI MoveTo в случайную точку в заданном диапазоне
  (Variables|Default|SetPreviosLocation (Transformation|GetActorLocation))
  (Variables|/Script/Engine.FloatingPawnMovement|SetMaxSpeed (Variables|Default|GetFloatingPawnMovement) (Variables|Default|GetSpeed))
  (CallFunction|MovetoPoint (Math|Random|RandomPointinBoundingBox "0, 0, 0" (Math|Vector|MakeVector (|(((Abs({FB4D8B70-4EC4-0B5F-75BD-5B8731465C87}))+(Abs({1ED38B1F-4DC4-F434-B221-8396986A2B4B})))/2)) (|(((Abs({2F66DE7D-4700-A58F-BFAA-8380BBD5154D}))+(Abs({672AA9A6-45E3-BEA2-7B3E-229BD895330A})))/2)) 0.0)) false 1e+01))

(fn ConstructionScript)